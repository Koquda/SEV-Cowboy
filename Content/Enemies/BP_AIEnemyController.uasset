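; BP_AIEnemyController is an enemy AI controller that chases the player's BP_Cowboy and keeps its pawn facing it.
; BeginPlay caches the first BP_Cowboy found, then calls FollowPlayer, which issues a single AI MoveTo toward it with debug prints for each outcome.
; Tick snaps the controlled pawn's yaw toward the cowboy every frame while that reference is valid.
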(event Custom|FollowPlayer
  (AI|AIMoveTo 0 "0, 0, 0" (Variables|Default|GetCowboyPlayer) 5.0 false
    (:then
      (Development|PrintString "On movement"))
    (:OnSuccess
      (Development|PrintString "Success"))
    (:OnFail
      (Development|PrintString "Fail"))))

(event EventBeginPlay
  (bind _returnvalue (Actor|GetActorOfClass "/Game/BP_Cowboy.BP_Cowboy_C"))
  (Variables|Default|SetCowboyPlayer _returnvalue)
  (CallFunction|FollowPlayer))

(event EventTick
  (params (DeltaSeconds :type Float%20%28single-precision%29))
  (bind _returnvalue (Pawn|GetControlledPawn))
  (bind _cowboyplayer (Variables|Default|GetCowboyPlayer)
    (:then
      (Transformation|SetActorRotation _returnvalue (Math|Rotator|MakeRotator 0.0 0.0 (.yaw (Math|Rotator|FindLookatRotation (Transformation|GetActorLocation _returnvalue) (Transformation|GetActorLocation _cowboyplayer))))))
    (:else)))

(fn ConstructionScript)