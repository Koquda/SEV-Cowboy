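; BP_ShootingComponent is a component that gives its owning actor a projectile shooting ability with a cooldown.
; Its Shoot event finds every ArrowComponent on the owner tagged "ShootingArrow" and spawns a ProjectileClass actor at each arrow's world transform, so tagged arrows act as muzzles.
; A DoOnce gate blocks further shots until a ShootingCooldown delay resets it.
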(event Custom|Shoot
  (Utilities|FlowControl|DoOnce false :!label _label
    (:Completed
      (Utilities|FlowControl|Sequence
        (:then_0
          (for _array_element (Actor|GetComponentsbyTag (Components|GetOwner) "/Script/Engine.ArrowComponent" "ShootingArrow")
            (bind _asarrow_component (Utilities|Casting|CastToArrowComponent _array_element))
            (Game|SpawnActorfromClass (Variables|Shooting|Projectiles|GetProjectileClass) (Transformation|GetWorldTransform _asarrow_component) "Undefined" 0 0)))
        (:then_1
          (Utilities|FlowControl|Delay (Variables|Shooting|GetShootingCooldown))
          (goto _label Reset))))))